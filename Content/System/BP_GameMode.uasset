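; BP_GameMode is a game mode that creates the player and boss HP bar widgets and adds them to the viewport.
; Setup runs once through a DoOnce on Tick rather than in BeginPlay, which is empty.
; Both widget references are stored, and only the player bar is initialized to full health.
; A disconnected search for Player-tagged ThirdPersonCharacter actors never runs.
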(event `self.ReceiveBeginPlay`)

(event `self.ReceiveTick`
  (params (DeltaSeconds :type "Float (single-precision)"))
  (`/Engine/EditorBlueprintResources/StandardMacros.DoOnce` false
    (:`Completed`
      (`|ExecutionSequence`
        (:`then_0`
          (bind _returnvalue (`|CreateWidget` "/Game/System/UI/Player/WBP_HPBar_Player.WBP_HPBar_Player_C"))
          (bind _output_get (set `self.HPBarPlayerWidget` _returnvalue))
          (`UserWidget.AddToViewport` _output_get 0)
          (`/Game/System/UI/Player/WBP_HPBar_Player.UpdateHP` (`self.HPBarPlayerWidget`) 1.0))
        (:`then_1`
          (bind _returnvalue_2 (`|CreateWidget` "/Game/System/UI/Enemy/WBP_HPBar_Boss.WBP_HPBar_Boss_C"))
          (bind _output_get_2 (set `self.HPBarBossWidget` _returnvalue_2))
          (`UserWidget.AddToViewport` _output_get_2 0))))))

(fn `UserConstructionScript`)