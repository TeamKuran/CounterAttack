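; Anim notify state that marks the window in an enemy animation during which BP_Enemy can be countered.
; On begin it casts the mesh owner to BP_Enemy, sets its CounterdFlg and swaps material slot 0 to CounterMat as a visual cue.
; On end it clears the flag and restores DefMat.
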(fn `Received_NotifyBegin`
  (params (MeshComp :type "SkeletalMeshComponent Object Reference") (Animation :type "AnimSequenceBase Object Reference") (TotalDuration :type "Float (double-precision)"))
  (returns (ReturnValue :type Boolean))
  (bind _asbp_enemy (cast `/Game/Kura/Enemy/BP_Enemy` (`ActorComponent.GetOwner` MeshComp)))
  (set `/Game/Kura/Enemy/BP_Enemy.CounterdFlg` true _asbp_enemy)
  (`PrimitiveComponent.SetMaterial` (`Character.Mesh` _asbp_enemy) 0 (`/Game/Kura/Enemy/BP_Enemy.CounterMat` _asbp_enemy))
  (return false))

(fn `Received_NotifyEnd`
  (params (MeshComp :type "SkeletalMeshComponent Object Reference") (Animation :type "AnimSequenceBase Object Reference"))
  (returns (ReturnValue :type Boolean))
  (bind _asbp_enemy (cast `/Game/Kura/Enemy/BP_Enemy` (`ActorComponent.GetOwner` MeshComp)))
  (set `/Game/Kura/Enemy/BP_Enemy.CounterdFlg` false _asbp_enemy)
  (`PrimitiveComponent.SetMaterial` (`Character.Mesh` _asbp_enemy) 0 (`/Game/Kura/Enemy/BP_Enemy.DefMat` _asbp_enemy))
  (return false))