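; Stationary sword-wielding enemy that slashes on a fixed timer, with no targeting or movement logic of its own (provisional attack).
; BeginPlay takes ownership of the child weapon to avoid self-damage, saves the default material for restoring counter-window tint, and caches the HP bar widget.
; Damage updates HP and the bar, then plays a hit reaction or a one-time death with sound, frozen animation and delayed destroy.
; A HitStop call remains unwired.
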(event `self.ReceiveBeginPlay`
  ;[1 1 1] 剣で自分がダメージを受けないようにする
  (`parent.ReceiveBeginPlay`)
  (`self.SetOwner` (`ChildActorComponent.ChildActor` (`self.WeaponActor`)) self)
  ;[1 1 1] カウンター可能時の色変えから戻る用にデフォルトのマテリアル保存
  (set `self.DefMat` (`PrimitiveComponent.GetMaterial` (`self.Mesh`) 0))
  ;[1 1 1] ウィジェットを参照するために変数にセットする
  (bind _aswbp_hpbar_wimps (cast `/Game/System/UI/Enemy/WBP_HPBar_Wimps` (`WidgetComponent.GetUserWidgetObject` (`self.Widget`))))
  (set `self.EnemyWBP` _aswbp_hpbar_wimps))

(event `self.ReceiveAnyDamage`
  (params (Damage :type "Float (single-precision)") (DamageType :type "DamageType Object Reference") (InstigatedBy :type "Controller Object Reference") (DamageCauser :type "Actor Object Reference"))
  ;[1 1 1] 攻撃を受けた場合の処理
  (bind _curhp (`self.UpdateHP` Damage))
  (`/Game/System/UI/Enemy/WBP_HPBar_Wimps.UpdateHP` (`self.EnemyWBP`) (/ _curhp (`self.MaxHealth`)))
  (if (> _curhp 0.0)
    ;;[1 1 1] HPがまだ残っている状態
    (`self.PlayAnimMontage` "/Game/Player/Animation/Player/Hit_To_Body_mixamo_com_Montage.Hit_To_Body_mixamo_com_Montage")
    (else
      ;;[1 1 1] 死んだ時
      (`/Engine/EditorBlueprintResources/StandardMacros.DoOnce` false
        (:`Completed`
          (`GameplayStatics.PlaySound2D` "/Game/Sound/SE/モンスター撃破__online-audio-converter_com_.モンスター撃破__online-audio-converter_com_" 1.0 1.0 0.0 null null)
          (bind _returnvalue (`self.PlayAnimMontage` "/Game/Player/Animation/Player/Sword_And_Shield_Death_mixamo_com_Montage.Sword_And_Shield_Death_mixamo_com_Montage"))
          (`KismetSystemLibrary.Delay` (- _returnvalue 0.27))
          (set `SkeletalMeshComponent.bPauseAnims` true (`self.Mesh`))
          (`CharacterMovementComponent.DisableMovement` (`self.CharacterMovement`))
          (`KismetSystemLibrary.Delay` _returnvalue)
          (`self.K2_DestroyActor`))))))

(event `self.ReceiveTick`
  (params (DeltaSeconds :type "Float (single-precision)"))
  ;[1 1 1] 敵の攻撃（仮）
  (bind _output_get (set `self.Timer` (+ DeltaSeconds (`self.Timer`))))
  (if (>= _output_get 3.0)
    (`self.PlayAnimMontage` "/Game/Kura/Enemy/ENEMY_SLASH_Montage.ENEMY_SLASH_Montage")
    (set `self.Timer` 0.0)))

(fn `UserConstructionScript`
  (bind _asbp_base_weapon (cast `/Game/Player/Animation/Player/Weapon/BP_BaseWeapon` (`ChildActorComponent.ChildActor` (`self.WeaponActor`))))
  (`KismetArrayLibrary.Array_Add` (`self.WeaponArry`) _asbp_base_weapon))