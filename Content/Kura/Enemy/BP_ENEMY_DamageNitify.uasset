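; Anim notify state that opens the enemy's sword damage window during an attack animation.
; On begin, it casts the mesh owner to BP_Enemy, gets its child-actor BP_BaseWeapon and calls SwordActive.
; On end, it follows the same path and calls SwordDeactive, so the weapon is active only for the notify's span.
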(fn `Received_NotifyBegin`
  (params (MeshComp :type "SkeletalMeshComponent Object Reference") (Animation :type "AnimSequenceBase Object Reference") (TotalDuration :type "Float (double-precision)"))
  (returns (ReturnValue :type Boolean))
  (bind _asbp_enemy (cast `/Game/Kura/Enemy/BP_Enemy` (`ActorComponent.GetOwner` MeshComp)))
  (bind _asbp_base_weapon (cast `/Game/ThirdPersonBP/Animation/Player/Weapon/BP_BaseWeapon` (`ChildActorComponent.ChildActor` (`/Game/Kura/Enemy/BP_Enemy.ChildActor` _asbp_enemy))))
  (`/Game/ThirdPersonBP/Animation/Player/Weapon/BP_BaseWeapon.SwordActive` _asbp_base_weapon)
  (return false))

(fn `Received_NotifyEnd`
  (params (MeshComp :type "SkeletalMeshComponent Object Reference") (Animation :type "AnimSequenceBase Object Reference"))
  (returns (ReturnValue :type Boolean))
  (bind _asbp_enemy (cast `/Game/Kura/Enemy/BP_Enemy` (`ActorComponent.GetOwner` MeshComp)))
  (bind _asbp_base_weapon (cast `/Game/ThirdPersonBP/Animation/Player/Weapon/BP_BaseWeapon` (`ChildActorComponent.ChildActor` (`/Game/Kura/Enemy/BP_Enemy.ChildActor` _asbp_enemy))))
  (`/Game/ThirdPersonBP/Animation/Player/Weapon/BP_BaseWeapon.SwordDeactive` _asbp_base_weapon)
  (return false))