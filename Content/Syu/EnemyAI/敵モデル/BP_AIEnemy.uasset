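; Enemy AI character with a melee slash, an HP bar widget and a child-actor weapon registered in its weapon array.
; Tick counts down a montage timer, then either slashes when the player is in close range, stopping AI logic, or restarts that logic.
; Damage updates HP and the bar, playing a hit montage while alive.
; Death runs once: sound, montage, paused pose and disabled movement, then delayed destruction.
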(event `self.ReceiveBeginPlay`
  (`parent.ReceiveBeginPlay`)
  ;[1 1 1] ウィジェットを参照するために変数にセットする
  (bind _aswbp_hpbar_wimps (cast `/Game/System/UI/Enemy/WBP_HPBar_Wimps` (`WidgetComponent.GetUserWidgetObject` (`self.Widget`))))
  (set `self.EnemyWBP` _aswbp_hpbar_wimps))

(event `self.ReceiveTick`
  (params (DeltaSeconds :type "Float (single-precision)"))
  (bind _returnvalue (- (`self.AnimTime`) DeltaSeconds))
  (if (> 0.0 _returnvalue)
    (set `self.AnimTime` 0.0)
    (else
      (set `self.AnimTime` _returnvalue)))
  (if (== (`self.AnimTime`) 0.0)
    (if (`self.Move`)
      (if (<= (`KismetMathLibrary.VSize` (- (`self.K2_GetActorLocation`) (`self.K2_GetActorLocation` (`GameplayStatics.GetPlayerPawn` 0)))) 200.0)
        ;[1 1 1] 攻撃処理
        (bind _returnvalue_2 (`self.PlayAnimMontage` "/Game/Kura/Enemy/ENEMY_SLASH_Montage.ENEMY_SLASH_Montage"))
        (set `self.AnimTime` _returnvalue_2)
        (set `self.Move` false)
        ;[1 1 1] AIの停止
        (`BrainComponent.StopLogic` (`AIController.BrainComponent` (`AIBlueprintHelperLibrary.GetAIController` self)) ""))
      (else
        ;[1 1 1] AI再開
        (`BrainComponent.RestartLogic` (`AIController.BrainComponent` (`AIBlueprintHelperLibrary.GetAIController` self)))
        (set `self.Move` true)))))

(event `self.AIPerception.OnTargetPerceptionUpdated`
  (params (Actor :type "Actor Object Reference") (Stimulus :type "AIStimulus Structure")))

(event `self.ReceiveAnyDamage`
  (params (Damage :type "Float (single-precision)") (DamageType :type "DamageType Object Reference") (InstigatedBy :type "Controller Object Reference") (DamageCauser :type "Actor Object Reference"))
  ;[1 1 1] 攻撃を受けた場合の処理
  (bind _curhp (`self.UpdateHP` Damage))
  (`/Game/System/UI/Enemy/WBP_HPBar_Wimps.UpdateHP` (`self.EnemyWBP`) (/ _curhp (`self.MaxHealth`)))
  (if (> _curhp 0.0)
    ;;[1 1 1] HPがまだ残っている状態
    (bind _returnvalue (`self.PlayAnimMontage` "/Game/Kura/Player/Animation/Player/Hit_To_Body_mixamo_com_Montage.Hit_To_Body_mixamo_com_Montage"))
    (set `self.AnimTime` _returnvalue)
    (else
      ;;[1 1 1] 死んだ時
      (`/Engine/EditorBlueprintResources/StandardMacros.DoOnce` false
        (:`Completed`
          (`GameplayStatics.PlaySound2D` "/Game/Sound/SE/モンスター撃破__online-audio-converter_com_.モンスター撃破__online-audio-converter_com_" 1.0 1.0 0.0 null null)
          ;;;[1 1 1] AIの停止
          (`BrainComponent.StopLogic` (`AIController.BrainComponent` (`AIBlueprintHelperLibrary.GetAIController` self)) "")
          (bind _returnvalue_2 (`self.PlayAnimMontage` "/Game/Kura/Player/Animation/Player/Sword_And_Shield_Death_mixamo_com_Montage.Sword_And_Shield_Death_mixamo_com_Montage"))
          (set `self.AnimTime` _returnvalue_2)
          (`KismetSystemLibrary.Delay` (- _returnvalue_2 0.27))
          (set `SkeletalMeshComponent.bPauseAnims` true (`self.Mesh`))
          (`CharacterMovementComponent.DisableMovement` (`self.CharacterMovement`))
          ;[1 1 1] AIの停止
          (`BrainComponent.StopLogic` (`AIController.BrainComponent` (`AIBlueprintHelperLibrary.GetAIController` self)) "")
          (`KismetSystemLibrary.Delay` _returnvalue_2)
          (`self.K2_DestroyActor`))))))

(fn `UserConstructionScript`
  (`parent.UserConstructionScript`)
  (bind _asbp_base_weapon (cast `/Game/Kura/Weapon/BP_BaseWeapon` (`ChildActorComponent.ChildActor` (`self.ChildActor`))))
  (`KismetArrayLibrary.Array_Add` (`self.WeaponArry`) _asbp_base_weapon))