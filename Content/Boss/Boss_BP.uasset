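; Boss actor that detects the player in front of it and spawns attacks for close and long range.
; Each Tick it line-traces forward over Distance1, then over Distance2 only if the first trace hits nothing.
; A hit on an actor tagged Player spawns Boss_Atk_BP at the boss's location, the same class for both ranges, with no cooldown.
; Debug trace lines and printed hit messages are left on.
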(event `self.ReceiveTick`
  (params (DeltaSeconds :type "Float (single-precision)"))
  (bind (_returnvalue_x _returnvalue_y _returnvalue_z) (`KismetMathLibrary.BreakVector` (`self.K2_GetActorLocation`)))
  (bind (_returnvalue_x_2 _returnvalue_y_2 _returnvalue_z_2) (`KismetMathLibrary.BreakVector` (`self.K2_GetActorLocation`)))
  (bind _returnvalue (+ (`self.K2_GetActorLocation`) (0.0 0.0 1.5) (0.0 0.0 0.0)))
  (bind _returnvalue_2 (+ (`self.K2_GetActorLocation`) (0.0 0.0 1.5) (0.0 0.0 0.0)))
  ;[1 1 1] プレイヤーの接近判定　（近距離攻撃）
  (bind (_outhit _returnvalue_3) (`KismetSystemLibrary.LineTraceSingle` :`Start` _returnvalue_2 :`End` (+ _returnvalue_2 (* (`self.GetActorForwardVector`) (`self.Distance1`))) :`TraceChannel` "TraceTypeQuery1" :`DrawDebugType` "ForDuration" :`DrawTime` 0.0))
  (if _returnvalue_3
    (if (`self.ActorHasTag` (`.HitActor` (`GameplayStatics.BreakHitResult` _outhit)) "Player")
      (`KismetSystemLibrary.PrintString` "Hit 1" true true (struct :`G` 0.66 :`B` 1.0 :`A` 1.0) 300.0)
      ;[1 1 1] アクターの自動生成　（近距離攻撃）
      (`|SpawnActorFromClass` "/Game/Boss/Boss_Atk_BP.Boss_Atk_BP_C" (`KismetMathLibrary.Conv_VectorToTransform` (`KismetMathLibrary.MakeVector` _returnvalue_x _returnvalue_y _returnvalue_z)) "Undefined" "OverrideRootScale" null null))
    (else
      ;[1 1 1] プレイヤーの接近判定　（遠距離攻撃）
      (bind (_outhit_2 _returnvalue_4) (`KismetSystemLibrary.LineTraceSingle` :`Start` _returnvalue :`End` (+ _returnvalue (* (`self.GetActorForwardVector`) (`self.Distance2`))) :`TraceChannel` "TraceTypeQuery1" :`DrawDebugType` "ForDuration" :`TraceColor` (struct :`G` 0.014294 :`B` 1.0 :`A` 1.0) :`DrawTime` 0.0))
      (if _returnvalue_4
        (if (`self.ActorHasTag` (`.HitActor` (`GameplayStatics.BreakHitResult` _outhit_2)) "Player")
          (`KismetSystemLibrary.PrintString` "Hit 2" true true (struct :`G` 0.66 :`B` 1.0 :`A` 1.0) 300.0)
          ;[1 1 1] アクターの自動生成　（遠距離攻撃）
          (`|SpawnActorFromClass` "/Game/Boss/Boss_Atk_BP.Boss_Atk_BP_C" (`KismetMathLibrary.Conv_VectorToTransform` (`KismetMathLibrary.MakeVector` _returnvalue_x_2 _returnvalue_y_2 _returnvalue_z_2)) "Undefined" "OverrideRootScale" null null))))))

(fn `UserConstructionScript`)