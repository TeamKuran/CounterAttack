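; BP_AI_Boss_Controller is the AI controller for a boss, driving it with the BT_Boss behavior tree and BB_Boss blackboard.
; On BeginPlay it sets up the blackboard and starts the tree.
; When perception updates, it writes each updated actor's first last-sensed stimulus result to the SensedFlag blackboard bool.
; All updated actors share that single flag, so the last one processed determines its value.
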(event `self.ReceiveBeginPlay`
  (`self.UseBlackboard` "/Game/ナビメッシュ/BB_Boss.BB_Boss")
  (`self.RunBehaviorTree` "/Game/ナビメッシュ/BT_Boss.BT_Boss"))

(event `self.AIPerception.OnPerceptionUpdated`
  (params (UpdatedActors :type "Array of Actor Object Reference (by ref)"))
  (for _array_element UpdatedActors
    (bind _info (`AIPerceptionComponent.GetActorsPerception` (`self.AIPerception`) _array_element))
    (`BlackboardComponent.SetValueAsBool` (`AIBlueprintHelperLibrary.GetBlackboard` null) "SensedFlag" (`.bSuccessfullySensed` (break `AIStimulus` (`|GetArrayItem` (`.LastSensedStimuli` (break `ActorPerceptionBlueprintInfo` _info))))))))

(fn `UserConstructionScript`)