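; BP_ProtBoss is a prototype boss enemy that takes damage, shows its health on a widget HP bar and dies at zero HP.
; Construction registers its child-actor weapon in a weapon array; BeginPlay sets weapon ownership, caches the HP bar and saves the default material for reverting the counter-window color change.
; AnyDamage updates the bar and, on death, runs a one-shot sequence: sound, frozen animation, stopped AI, then delayed movement disable and destruction.
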(event `self.ReceiveBeginPlay`
  (`parent.ReceiveBeginPlay`)
  (`self.SetOwner` (`ChildActorComponent.ChildActor` (`self.WeaponActor`)) self)
  ;[1 1 1] カウンター可能時の色変えから戻る用にデフォルトのマテリアル保存
  (set `self.DefMat` (`PrimitiveComponent.GetMaterial` (`self.Mesh`) 0))
  ;[1 1 1] ウィジェットを参照するために変数にセットする
  (bind _aswbp_hpbar_wimps (cast `/Game/Features/UI/Blueprints/System/UI/Enemy/WBP_HPBar_Wimps` (`WidgetComponent.GetUserWidgetObject` (`self.Widget`))))
  (set `self.EnemyWBP` _aswbp_hpbar_wimps))

(event `self.ReceiveAnyDamage`
  (params (Damage :type "Float (single-precision)") (DamageType :type "DamageType Object Reference") (InstigatedBy :type "Controller Object Reference") (DamageCauser :type "Actor Object Reference"))
  ;[1 1 1] 攻撃を受けた場合の処理
  (bind _curhp (`self.UpdateHP` Damage))
  (`/Game/Features/UI/Blueprints/System/UI/Enemy/WBP_HPBar_Wimps.UpdateHP` (`self.EnemyWBP`) (/ _curhp (`self.MaxHealth`)))
  (if (not (> _curhp 0.0))
    ;;[1 1 1] 死んだ時
    (`/Engine/EditorBlueprintResources/StandardMacros.DoOnce` false
      (:`Completed`
        (`GameplayStatics.PlaySound2D` "/Game/Main/Common/Sound/SE/モンスター撃破__online-audio-converter_com_.モンスター撃破__online-audio-converter_com_" 1.0 1.0 0.0 null null)
        (set `SkeletalMeshComponent.bPauseAnims` true (`self.Mesh`))
        (`BrainComponent.StopLogic` (`AIController.BrainComponent` (`AIBlueprintHelperLibrary.GetAIController` self)) "")
        (`KismetSystemLibrary.Delay` 1.0)
        (`CharacterMovementComponent.DisableMovement` (`self.CharacterMovement`))
        (`KismetSystemLibrary.Delay` 1.0)
        (`self.K2_DestroyActor`)))))

(fn `UserConstructionScript`
  (`parent.UserConstructionScript`)
  (bind _asbp_base_weapon (cast `/Game/Features/Player/Weapon/BP_BaseWeapon` (`ChildActorComponent.ChildActor` (`self.WeaponActor`))))
  (`KismetArrayLibrary.Array_Add` (`self.WeaponArry`) _asbp_base_weapon))