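; AI controller for the flying boss that runs its behavior tree and feeds it perception data.
; On BeginPlay it sets up BB_FlyBoss, runs BT_FlyBoss and flags the boss as flying.
; When AI Perception updates, it filters for the player character and writes whether the first last-sensed stimulus succeeded into the SensedFlag blackboard key.
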(event `self.ReceiveBeginPlay`
  (bind _blackboardcomponent (`self.UseBlackboard` "/Game/Features/Boss/Blueprints/ナビメッシュ/BOSS_2/BB_FlyBoss.BB_FlyBoss"))
  (`self.RunBehaviorTree` "/Game/Features/Boss/Blueprints/ナビメッシュ/BOSS_2/BT_FlyBoss.BT_FlyBoss")
  (`BlackboardComponent.SetValueAsBool` _blackboardcomponent "isFlying" true))

(event `self.AIPerception.OnPerceptionUpdated`
  (params (UpdatedActors :type "Array of Actor Object Reference (by ref)"))
  (for _array_element UpdatedActors
    (if (== _array_element (`GameplayStatics.GetPlayerCharacter` 0))
      (bind _info (`AIPerceptionComponent.GetActorsPerception` (`self.AIPerception`) _array_element))
      (`BlackboardComponent.SetValueAsBool` (`AIBlueprintHelperLibrary.GetBlackboard` self) "SensedFlag" (`.bSuccessfullySensed` (break `AIStimulus` (`|GetArrayItem` (`.LastSensedStimuli` (break `ActorPerceptionBlueprintInfo` _info)))))))))

(fn `UserConstructionScript`)