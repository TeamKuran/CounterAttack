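; Flying boss character that starts in flying movement and shows the GameMode's boss HP bar, hiding it on death.
; A hit from a returned thunder ball grounds it by clearing the isFlying blackboard key, switching to NavWalking and setting gravity.
; Normal, special and bullet attack overrides call the parent, then play fly-boss montages.
; SpawnBullet fires the given class from a mesh socket, aimed at the player.
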(event `self.ReceiveBeginPlay`
  (bind _charactermovement (`self.CharacterMovement`))
  (`parent.ReceiveBeginPlay`)
  ;[1 1 1] ゲームモードをキャストして参照変数に格納し、そこからテスト用のプレイヤーＨＰバーを取り出して格納する
  (`KismetSystemLibrary.Delay` 0.1)
  (bind _asbp_game_mode (cast `/Game/Main/Common/Bluprints/BP_GameMode` (`GameplayStatics.GetGameMode`)))
  (bind _hpbarbosswidget (`/Game/Main/Common/Bluprints/BP_GameMode.HPBarBossWidget` _asbp_game_mode))
  (bind _output_get (set `self.WBP_HPBarRef` _hpbarbosswidget))
  (`Widget.SetVisibility` _output_get "Visible")
  (`UserWidget.PlayAnimation` _hpbarbosswidget (`/Game/Features/UI/Blueprints/Enemy/WBP_HPBar_Boss.In` _hpbarbosswidget) 0.0 1 "Forward" 1.0 false)
  ;[1 1 1] ＨＰBarにＨＰを反映
  (`self.UpdateHealthBar`)
  (`CharacterMovementComponent.SetMovementMode` _charactermovement "MOVE_Flying" 0)
  (set `CharacterMovementComponent.DefaultLandMovementMode` "MOVE_Flying" _charactermovement))

(event `self.ReceiveTick`
  (params (DeltaSeconds :type "Float (single-precision)"))
  (`parent.ReceiveTick` DeltaSeconds))

(event `self.DamagedAliveEvent`
  (params (DamageCauser :type "Actor Object Reference"))
  (bind _charactermovement (`self.CharacterMovement`))
  (cast `/Game/Features/Boss/Blueprints/Boss/ACBP_ThunderBallReturn` DamageCauser)
  (`BlackboardComponent.SetValueAsBool` (`AIBlueprintHelperLibrary.GetBlackboard` null) "isFlying" false)
  (`CharacterMovementComponent.SetMovementMode` _charactermovement "MOVE_NavWalking" 0)
  (set `CharacterMovementComponent.DefaultLandMovementMode` "MOVE_NavWalking" _charactermovement)
  (set `CharacterMovementComponent.GravityScale` 1.0 _charactermovement))

(event `/Game/Features/Enemy/CBP_BaseEnemy.DamagedDeadEvent`
  (`Widget.SetVisibility` (`self.WBP_HPBarRef`) "Collapsed")
  (`parent.DamagedDeadEvent`))

(fn `BulletAttack`
  (`parent.BulletAttack`)
  (`self.PlayAnimMontage` "/Game/Features/Boss/Blueprints/アニメーション/Master_2/Boss_Fly_Bullet_Anim_Montage.Boss_Fly_Bullet_Anim_Montage"))

(fn `NormalAttack`
  (`parent.NormalAttack`)
  (`self.PlayAnimMontage` "/Game/Features/Boss/Blueprints/アニメーション/Master_2/Boss_Fly_tuki_Anim_Montage.Boss_Fly_tuki_Anim_Montage" 2.0))

(fn `SpawnBullet`
  (params (NewParam :type "Actor Class Reference"))
  (returns (Bullet :type "Actor Object Reference"))
  (bind _returnvalue_location (`KismetMathLibrary.BreakTransform` (`SceneComponent.GetSocketTransform` (`self.Mesh`) "Bulletソケット" "RTS_World")))
  (bind _returnvalue (`|SpawnActorFromClass` NewParam (`KismetMathLibrary.MakeTransform` _returnvalue_location (`KismetMathLibrary.FindLookAtRotation` _returnvalue_location (`self.K2_GetActorLocation` (`GameplayStatics.GetPlayerCharacter` 0)))) "Undefined" "OverrideRootScale" self null))
  (return _returnvalue))

(fn `SpecialAttack`
  (`parent.SpecialAttack`)
  (`self.PlayAnimMontage` "/Game/Features/Boss/Blueprints/アニメーション/Master_2/Boss_Fly_tossin_Anim_Montage.Boss_Fly_tossin_Anim_Montage"))

(fn `UserConstructionScript`
  (`parent.UserConstructionScript`))