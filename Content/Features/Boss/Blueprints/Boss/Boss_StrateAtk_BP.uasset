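; Boss straight-shot projectile that flies in a fixed line toward where the player was when it spawned.
; BeginPlay caches the normalized direction to player pawn 0, and Tick moves the actor along it by Speed per frame without sweep or delta-time scaling.
; On sphere overlap it damages the player and plays a hit sound.
; It then destroys itself after a short delay, as it does on overlapping anything except its owner.
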(event `self.ReceiveBeginPlay`
  (set `self.TargetVec` (`KismetMathLibrary.Normal` (- (`self.K2_GetActorLocation` (`GameplayStatics.GetPlayerPawn` 0)) (`self.K2_GetActorLocation`)))))

(event `self.ReceiveTick`
  (params (DeltaSeconds :type "Float (single-precision)"))
  (`self.K2_SetActorLocation` (+ (`self.K2_GetActorLocation`) (* (`self.TargetVec`) (`self.Speed`)))))

(event `self.Sphere.OnComponentBeginOverlap`
  (params (OverlappedComponent :type "PrimitiveComponent Object Reference") (OtherActor :type "Actor Object Reference") (OtherComp :type "PrimitiveComponent Object Reference") (OtherBodyIndex :type Integer) (bFromSweep :type Boolean) (SweepResult :type "HitResult Structure (by ref)"))
  (bind _returnvalue (`GameplayStatics.GetPlayerPawn` 0))
  (if (== OtherActor _returnvalue)
    (`GameplayStatics.ApplyDamage` _returnvalue (`self.Damage`) null self)
    (`GameplayStatics.PlaySoundAtLocation` "/Game/Features/Sound/Sozai/SE/SE_Player_Damage_Cue.SE_Player_Damage_Cue" (`self.K2_GetActorLocation`) (struct) 1.0 1.0 0.0 null null null)
    (`KismetSystemLibrary.Delay` 0.1)
    (`self.K2_DestroyActor` :!label _label)
    (elif (!= OtherActor (`self.GetOwner`))
      (`KismetSystemLibrary.Delay` 0.1)
      (goto _label))))

(fn `UserConstructionScript`)