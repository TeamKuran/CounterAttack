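; Sword Machine boss character that supplies boss-specific attacks and HUD hookup on top of its parent class.
; Normal, special and bullet attacks each call the parent and play their own montage, while SpawnBullet fires an enemy bullet aimed at player 0.
; HitEvent replaces the parent logic by calling NextSection on the boss AnimBP.
; The GameMode's boss HP bar animates in after a short BeginPlay delay and collapses on death.
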(event `self.ReceiveBeginPlay`
  (`parent.ReceiveBeginPlay`)
  ;[1 1 1] ゲームモードをキャストして参照変数に格納し、そこからテスト用のプレイヤーＨＰバーを取り出して格納する
  (`KismetSystemLibrary.Delay` 0.1)
  (bind _asbp_game_mode (cast `/Game/Features/UI/BP_GameMode` (`GameplayStatics.GetGameMode`)))
  (bind _hpbarbosswidget (`/Game/Features/UI/BP_GameMode.HPBarBossWidget` _asbp_game_mode))
  (bind _output_get (set `self.WBP_HPBarRef` _hpbarbosswidget))
  (`Widget.SetVisibility` _output_get "Visible")
  (`UserWidget.PlayAnimation` _hpbarbosswidget (`/Game/Features/UI/Blueprints/Enemy/WBP_HPBar_Boss.In` _hpbarbosswidget) 0.0 1 "Forward" 1.0 false)
  ;[1 1 1] ＨＰBarにＨＰを反映
  (`self.UpdateHealthBar`))

(event `self.ReceiveTick`
  (params (DeltaSeconds :type "Float (single-precision)"))
  (`parent.ReceiveTick` DeltaSeconds))

(event `/Game/Features/Enemy/CBP_BaseEnemy.DamagedDeadEvent`
  (`Widget.SetVisibility` (`self.WBP_HPBarRef`) "Collapsed")
  (`parent.DamagedDeadEvent`))

(fn `BulletAttack`
  (`parent.BulletAttack`)
  (`self.PlayAnimMontage` "/Game/Features/Boss/Blueprints/アニメーション/hassya_Anim_Montage.hassya_Anim_Montage"))

(fn `HitEvent`
  (bind _asabp_smboss_animetion (cast `/Game/Features/Boss/Blueprints/アニメーション/ABP_SMBossAnimetion` (`SkeletalMeshComponent.GetAnimInstance` (`self.Mesh`))))
  (`/Game/Features/Boss/Blueprints/アニメーション/ABP_SMBossAnimetion.NextSection` _asabp_smboss_animetion))

(fn `NormalAttack`
  (`parent.NormalAttack`)
  (`self.PlayAnimMontage` "/Game/Features/Boss/Blueprints/アニメーション/kaiten01_Anim_Montage.kaiten01_Anim_Montage"))

(fn `SpawnBullet`
  (params (NewParam :type "Actor Class Reference"))
  (returns (Bullet :type "Actor Object Reference"))
  (bind _returnvalue (`self.GetTransform` self))
  (bind _returnvalue_2 (`KismetMathLibrary.MakeVector` (.x (.location _returnvalue)) (.y (.location _returnvalue)) (+ (.z (.location _returnvalue)) 0.0)))
  (bind _returnvalue_3 (`|SpawnActorFromClass` "/Game/Features/Enemy/EnemyAI/敵モデル/ACBP_EnemyBullet.ACBP_EnemyBullet_C" (`KismetMathLibrary.MakeTransform` _returnvalue_2 (`KismetMathLibrary.FindLookAtRotation` _returnvalue_2 (`self.K2_GetActorLocation` (`GameplayStatics.GetPlayerCharacter` 0)))) "Undefined" "OverrideRootScale" self null))
  (return _returnvalue_3))

(fn `SpecialAttack`
  (`parent.SpecialAttack`)
  (`self.PlayAnimMontage` "/Game/Features/Boss/Blueprints/アニメーション/tossin_NoRoot_Anim_Montage.tossin_NoRoot_Anim_Montage"))

(fn `UserConstructionScript`
  (`parent.UserConstructionScript`))