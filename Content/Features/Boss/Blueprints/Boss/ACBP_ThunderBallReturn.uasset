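; Boss thunder ball projectile that a player's weapon can knock back toward its current owner.
; A player weapon overlap redirects it at max speed toward that owner, makes the player its owner, flips its team and recolors the Niagara effect.
; Otherwise, overlapping a non-invincible character of the opposing team deals damage with hit effect and sound.
; A DoOnce with a half-second delayed reset throttles repeat hits, as the ball is not destroyed here.
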(event `self.ReceiveBeginPlay`
  (bind _ascbp_base_charactor (cast `/Game/Features/Player/CBP_BaseCharactor` (`self.GetOwner`)))
  (set `self.PlayerorEnemy` (`/Game/Features/Player/CBP_BaseCharactor.PlayerOrEnemy` _ascbp_base_charactor)))

(event `self.SphereCollosion.OnComponentBeginOverlap`
  (params (OverlappedComponent :type "PrimitiveComponent Object Reference") (OtherActor :type "Actor Object Reference") (OtherComp :type "PrimitiveComponent Object Reference") (OtherBodyIndex :type Integer) (bFromSweep :type Boolean) (SweepResult :type "HitResult Structure (by ref)"))
  (bind _returnvalue (`self.GetOwner`))
  ;[1 1 1] overlapした時に自分の親アクタ以外だった場合、applydamageで敵にダメージを与える
  (bind _asacbp_base_weapon (cast `/Game/Features/Player/Weapon/ACBP_BaseWeapon` OtherActor)
    (:`then`
      (bind _ascbp_base_charactor (cast `/Game/Features/Player/CBP_BaseCharactor` (`self.GetOwner` _asacbp_base_weapon)))
      (if (`|EnumEquality` (`/Game/Features/Player/CBP_BaseCharactor.PlayerOrEnemy` _ascbp_base_charactor) "NewEnumerator0")
        (set `MovementComponent.Velocity` (* (`KismetMathLibrary.Normal` (- (`self.K2_GetActorLocation` (`self.GetOwner`)) (`self.K2_GetActorLocation`))) (`ProjectileMovementComponent.MaxSpeed` (`self.ProjectileMovement`))) (`self.ProjectileMovement`))
        (`self.SetOwner` _ascbp_base_charactor)
        (switch `/Game/Features/Player/E_PlayerOrEnemy` (`self.PlayerorEnemy`)
          (:`NewEnumerator0`
            (set `self.PlayerorEnemy` "NewEnumerator1")
            (`NiagaraComponent.SetNiagaraVariableLinearColor` (`self.Niagara`) "User_Color" (make `LinearColor` 2.0 1.0 0.0 1.0)))
          (:`NewEnumerator1`
            (set `self.PlayerorEnemy` "NewEnumerator0")
            (`NiagaraComponent.SetNiagaraVariableLinearColor` (`self.Niagara`) "User_Color" (make `LinearColor` 0.0 1.0 2.0 1.0))))))
    (:`CastFailed`
      (if (!= OtherActor _returnvalue)
        (bind _ascbp_base_charactor_2 (cast `/Game/Features/Player/CBP_BaseCharactor` OtherActor))
        (cast `/Game/Features/Player/CBP_BaseCharactor` _returnvalue)
        (if (`|EnumInequality` (`self.PlayerorEnemy`) (`/Game/Features/Player/CBP_BaseCharactor.PlayerOrEnemy` _ascbp_base_charactor_2))
          (if (not (`/Game/Features/Player/CBP_BaseCharactor.InvicibleFlg` _ascbp_base_charactor_2))
            (`/Engine/EditorBlueprintResources/StandardMacros.DoOnce` false :!label _label
              (:`Completed`
                (`GameplayStatics.ApplyDamage` OtherActor (`self.BulletDamage`) null self)
                (`NiagaraFunctionLibrary.SpawnSystemAtLocation` "/Game/Features/Player/Effect/0510/FX/FX_Hit.FX_Hit" (`self.K2_GetActorLocation`))
                (`GameplayStatics.PlaySound2D` "/Game/Features/Sound/Sozai/SE/SE_Hit_Cue.SE_Hit_Cue" 1.0 1.0 0.0 null null)
                (`KismetSystemLibrary.Delay` 0.5)
                (goto _label :!via `Reset`)))))))))

(fn `UserConstructionScript`)