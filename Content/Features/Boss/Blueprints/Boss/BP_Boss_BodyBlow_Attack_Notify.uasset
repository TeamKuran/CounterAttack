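; Animation notify state for a boss body blow attack that makes the boss leap toward the player.
; When the notify begins, it casts the mesh owner to BP_BaseBoss and takes the normalized direction to player 0.
; It keeps that direction's X and Y, forces Z to 1, scales the vector and launches the boss, overriding its current velocity.
; Notify end has no behavior.
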(fn `Received_NotifyBegin`
  (params (MeshComp :type "SkeletalMeshComponent Object Reference") (Animation :type "AnimSequenceBase Object Reference") (TotalDuration :type "Float (double-precision)"))
  (returns (ReturnValue :type Boolean))
  (bind _returnvalue (`ActorComponent.GetOwner` MeshComp))
  (bind (_returnvalue_x _returnvalue_y) (`KismetMathLibrary.BreakVector` (`KismetMathLibrary.Normal` (- (`Actor.K2_GetActorLocation` (`GameplayStatics.GetPlayerCharacter` MeshComp)) (`Actor.K2_GetActorLocation` _returnvalue)))))
  (bind _asbp_base_boss (cast `/Game/Features/Boss/Blueprints/Boss/BP_BaseBoss` _returnvalue))
  (`Character.LaunchCharacter` _asbp_base_boss (* (`KismetMathLibrary.MakeVector` _returnvalue_x _returnvalue_y 1.0) 500.0) true true)
  (return false))

(fn `Received_NotifyEnd`
  (params (MeshComp :type "SkeletalMeshComponent Object Reference") (Animation :type "AnimSequenceBase Object Reference"))
  (returns (ReturnValue :type Boolean))
  (return false))