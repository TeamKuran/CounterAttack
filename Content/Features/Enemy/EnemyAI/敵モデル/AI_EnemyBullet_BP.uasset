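; Enemy bullet actor that damages characters its collision sphere overlaps.
; On overlap it skips its owner and acts only on CBP_CharactorBase characters that are not invincible, applying damage, a burst effect and a hit sound.
; An optional FlyAway flag sends the victim flying relative to the owner, then clears.
; A DoOnce with a short delayed reset throttles repeat hits; the bullet is never destroyed here.
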(event `self.ReceiveBeginPlay`)

(event `self.SphereCollosion.OnComponentBeginOverlap`
  (params (OverlappedComponent :type "PrimitiveComponent Object Reference") (OtherActor :type "Actor Object Reference") (OtherComp :type "PrimitiveComponent Object Reference") (OtherBodyIndex :type Integer) (bFromSweep :type Boolean) (SweepResult :type "HitResult Structure (by ref)"))
  (bind _returnvalue (`self.GetOwner`))
  ;[1 1 1] overlapした時に自分の親アクタ以外だった場合、applydamageで敵にダメージを与える
  (if (!= OtherActor _returnvalue)
    (bind _ascbp_charactor_base (cast `/Game/Features/Player/Player_Main/CBP_CharactorBase` OtherActor))
    (if (not (`/Game/Features/Player/Player_Main/CBP_CharactorBase.InvicibleFlg` _ascbp_charactor_base))
      (`/Engine/EditorBlueprintResources/StandardMacros.DoOnce` false :!label _label
        (:`Completed`
          (`GameplayStatics.ApplyDamage` OtherActor (`self.BulletDamage`) null self)
          (`NiagaraFunctionLibrary.SpawnSystemAtLocation` "/Game/Main/Common/Niagara/HitEffect/FX/FX_Burst.FX_Burst" (`self.K2_GetActorLocation`))
          (if (`self.FlyAway`)
            (`/Game/Features/Player/MacroLiblary/Macro.FlyAway` OtherActor _returnvalue
              (:`Out`
                (set `self.FlyAway` false))))
          (`GameplayStatics.PlaySound2D` "/Game/Main/Common/Sound/SE/Cut01-1__online-audio-converter_com_.Cut01-1__online-audio-converter_com_" 1.0 1.0 0.0 null null)
          (`KismetSystemLibrary.Delay` 0.5)
          (goto _label :!via `Reset`))))))

(fn `UserConstructionScript`)