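; Stationary-named enemy Blueprint that plays a slash montage every three seconds from a Tick timer, marked as a provisional attack.
; BeginPlay owns the child-actor weapon to avoid self-damage and caches the default material for restoring after counter tinting; construction registers the weapon in an array.
; AnyDamage only calls UpdateHP.
; Hit reaction, death sequence and damage-scaled hit stop remain in disconnected, never-run nodes.
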(event `self.ReceiveBeginPlay`
  ;[1 1 1] 剣で自分がダメージを受けないようにする
  (`parent.ReceiveBeginPlay`)
  (`self.SetOwner` (`ChildActorComponent.ChildActor` (`self.WeaponActor`)) self)
  ;[1 1 1] カウンター可能時の色変えから戻る用にデフォルトのマテリアル保存
  (set `self.DefMat` (`PrimitiveComponent.GetMaterial` (`self.Mesh`) 0)))

(event `self.ReceiveAnyDamage`
  (params (Damage :type "Float (single-precision)") (DamageType :type "DamageType Object Reference") (InstigatedBy :type "Controller Object Reference") (DamageCauser :type "Actor Object Reference"))
  ;[1 1 1] 攻撃を受けた場合の処理
  (bind _curhp (`self.UpdateHP` Damage)))

(event `self.ReceiveTick`
  (params (DeltaSeconds :type "Float (single-precision)"))
  ;[1 1 1] 敵の攻撃（仮）
  (bind _output_get (set `self.Timer` (+ DeltaSeconds (`self.Timer`))))
  (if (>= _output_get 3.0)
    (`self.PlayAnimMontage` "/Game/Features/Enemy/Common/Animation/ENEMY_SLASH_Montage.ENEMY_SLASH_Montage")
    (set `self.Timer` 0.0)))

(fn `UserConstructionScript`
  (bind _asacbp_base_weapon (cast `/Game/Features/Player/Weapon/ACBP_BaseWeapon` (`ChildActorComponent.ChildActor` (`self.WeaponActor`))))
  (`KismetArrayLibrary.Array_Add` (`self.WeaponArry`) _asacbp_base_weapon))