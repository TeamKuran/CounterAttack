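; TPlayer_BP is an actor, apparently the title-screen player, that animates a material effect on its mesh.
; Tick calls Play on a timeline, whose track drives the "Power" scalar parameter on the mesh's materials.
; A NearlyActor helper compares two actors' distances to this one and returns the farther one, despite its name, but is not called in these graphs.
; BeginPlay, overlap and construction logic are empty.
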(event `self.ReceiveTick`
  (params (DeltaSeconds :type "Float (single-precision)"))
  (bind (_direction `_新規track_0`) (`Timeline|タイムライン_0` :`NewTime` 5.0)
    (:`Update`
      (`MeshComponent.SetScalarParameterValueOnMaterials` (`self.Mesh`) "Power" `_新規track_0`))))

(event `self.ReceiveBeginPlay`)

(fn `NearlyActor`
  (params (ActorA :type "Actor Object Reference") (ActorB :type "Actor Object Reference"))
  (returns (NearlyActor :type "Actor Object Reference"))
  (if (>= (`KismetMathLibrary.VSize` (- (`self.K2_GetActorLocation` ActorA) (`self.K2_GetActorLocation`))) (`KismetMathLibrary.VSize` (- (`self.K2_GetActorLocation` ActorB) (`self.K2_GetActorLocation`))))
    (return ActorA)
    (else
      (return ActorB))))

(fn `UserConstructionScript`)