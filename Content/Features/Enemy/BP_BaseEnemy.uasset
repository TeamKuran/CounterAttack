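; BP_BaseEnemy is a base enemy Blueprint that holds health and a mesh material for enemies.
; On BeginPlay it stores a dynamic instance of the mesh's first material in DefMat and sets Health to MaxHealth.
; UpdateHP subtracts a damage-or-heal amount, clamps only at zero and returns the new Health.
; Attack is an empty function, and Tick and overlap events are unused.
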(event `self.ReceiveBeginPlay`
  (bind _returnvalue (`PrimitiveComponent.CreateDynamicMaterialInstance` (`self.Mesh`) 0 null "None"))
  (set `self.DefMat` _returnvalue)
  (set `self.Health` (`self.MaxHealth`)))

(fn `Attack`)

(fn `UpdateHP`
  (params (DamageOrHeal :type "Float (double-precision)"))
  (returns (CurHP :type "Float (double-precision)"))
  (bind _returnvalue (- (`self.Health`) DamageOrHeal))
  (if (>= _returnvalue 0.0)
    (set `self.Health` _returnvalue)
    (else
      (set `self.Health` 0.0)))
  (return (`self.Health`)))

(fn `UserConstructionScript`)