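; Room wave spawner that starts enemy waves when the player first overlaps it and runs the game-clear flow.
; Spawns enemies from WaveInfoArray at target actors, updating a wave widget; enemies report deaths through DecreaseEnemyCount, triggering the next wave after a delay.
; The last wave also starts BP_SystemSpawnInfinity spawners from "InfinityInfo"-tagged wave infos.
; Once counted enemies are gone, it destroys those spawners and remaining enemies, plays the clear sequence, then restarts.
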(event `self.ReceiveBeginPlay`
  (bind _systemspawnwidget (`self.SystemSpawnWidget`))
  (set `self.FieldEnemyCount` 0) ; レベル上の敵の数初期化
  (set `self.WaveTotal` (`KismetArrayLibrary.Array_Length` (`self.WaveInfoArray`))) ; すべてのウェーブの数の合計
  (set `self.SpawnWaveIndex` 0) ; 現在のウェーブの番号初期化
  (bind _returnvalue (`|CreateWidget` "/Game/Features/System/Blueprints/SpawnWave/UMG_SystemSpawnWave.UMG_SystemSpawnWave_C"))
  (bind _output_get (set `self.SystemSpawnWidget` _returnvalue))
  (`UserWidget.AddToViewport` _output_get 0)
  (`/Game/Features/System/Blueprints/SpawnWave/UMG_SystemSpawnWave.SetWaveTotal` _systemspawnwidget (`self.WaveTotal`))
  (`/Game/Features/System/Blueprints/SpawnWave/UMG_SystemSpawnWave.SetWaveIndex` _systemspawnwidget (+ (`self.SpawnWaveIndex`) 1)))

(event `self.ReceiveActorBeginOverlap`
  (params (OtherActor :type "Actor Object Reference"))
  ;[1 1 1] プレイヤーが部屋に入ったら、最初のウェーブを開始する
  (if (== OtherActor (`GameplayStatics.GetPlayerPawn` 0))
    (`/Engine/EditorBlueprintResources/StandardMacros.DoOnce` false
      (:`Completed`
        (`self.SpawnWave` (`self.SpawnWaveIndex`))))))

(event `DecreaseEnemyCount`
  ;[1 1 1] 敵カウントを1減少させる
  (bind _result (`/Engine/EditorBlueprintResources/StandardMacros.DecrementInt` (`self.FieldEnemyCount`))
    (:`  `
      ;[1 1 1] レベル上に敵が存在しなくなったら、敵を生成する
      (if (== _result 0)
        (`KismetSystemLibrary.Delay` 3.0)
        (`self.SpawnWave` (`self.SpawnWaveIndex`))))))

(event `SpawnWave`
  (params (Index :type Integer))
  (`|ExecutionSequence`
    (:`then_0`
      ;[1 1 1] UMGに表示する数値を編集する
      (if (not (`self.IsLast`))
        (`/Game/Features/System/Blueprints/SpawnWave/UMG_SystemSpawnWave.SetWaveIndex` (`self.SystemSpawnWidget`) (+ (`self.SpawnWaveIndex`) 1))))
    (:`then_1`
      (if (not (`self.IsLast`))
        ;[1 1 1] 指定された配列番号のウェーブを呼び出し、敵を生成する(レベル上の敵をループ分増加させる)
        (for _array_element (`/Game/Features/System/Blueprints/SpawnWave/BP_WaveInfo.SpawnEnemyInfo` (`|GetArrayItem` (`self.WaveInfoArray`) Index))
          (bind (_enemytype _enemytransformtarget) (break `/Game/Features/System/Blueprints/SpawnWave/ST_SpawnEnemyInfo` _array_element))
          (if (`KismetSystemLibrary.IsValidClass` _enemytype)
            (if (`KismetSystemLibrary.IsValid` _enemytransformtarget)
              (bind _returnvalue (`|SpawnActorFromClass` _enemytype (`self.GetTransform` _enemytransformtarget) "Undefined" "OverrideRootScale" null null))
              (`Pawn.SpawnDefaultController` _returnvalue)
              (`/Engine/EditorBlueprintResources/StandardMacros.IncrementInt` (`self.FieldEnemyCount`)
                (:`  `
                  (set `/Game/Features/Enemy/CBP_BaseEnemy.SpawnType` "NewEnumerator1" _returnvalue))))))
        (`/Game/Features/System/Blueprints/SpawnWave/UMG_SystemSpawnWave.フェード` (`self.SystemSpawnWidget`))))
    (:`then_2`
      ;[1 1 1] 次に生成するウェーブ番号を格納する
      (if (== (`KismetArrayLibrary.Array_LastIndex` (`self.WaveInfoArray`)) (`self.SpawnWaveIndex`))
        (set `self.IsLast` true)
        (bind _outactors (`GameplayStatics.GetAllActorsWithTag` "InfinityInfo"))
        (for _array_element_2 _outactors
          (bind _asbp_wave_info (cast `/Game/Features/System/Blueprints/SpawnWave/BP_WaveInfo` _array_element_2))
          (bind _returnvalue_2 (`|SpawnActorFromClass` "/Game/Features/System/Blueprints/SpawnInfinity/BP_SystemSpawnInfinity.BP_SystemSpawnInfinity_C" (`self.GetTransform`) "Undefined" "OverrideRootScale" null null))
          (set `/Game/Features/System/Blueprints/SpawnInfinity/BP_SystemSpawnInfinity.WaveInfo` _asbp_wave_info _returnvalue_2)
          (`/Game/Features/System/Blueprints/SpawnInfinity/BP_SystemSpawnInfinity.SpawnWave` _returnvalue_2))
        (else
          (`/Engine/EditorBlueprintResources/StandardMacros.IncrementInt` (`self.SpawnWaveIndex`)))))
    (:`then_3`
      ;[1 1 1] すべてのウェーブが終わり、レベル上にすべての敵がいなくなったらゲームクリア
      (if (`self.IsLast`)
        (if (== (`self.FieldEnemyCount`) 0)
          (`self.GameClear`)
          (`|ExecutionSequence`
            (:`then_0`
              (bind _outactors_2 (`GameplayStatics.GetAllActorsOfClass` "/Game/Features/System/Blueprints/SpawnInfinity/BP_SystemSpawnInfinity.BP_SystemSpawnInfinity_C"))
              (for _array_element_3 _outactors_2
                (`self.K2_DestroyActor` _array_element_3)))
            (:`then_1`
              (bind _outactors_3 (`GameplayStatics.GetAllActorsOfClass` "/Game/Features/Enemy/CBP_BaseEnemy.CBP_BaseEnemy_C"))
              (for _array_element_4 _outactors_3
                (`self.K2_DestroyActor` _array_element_4)))))))))

(event `GameClear`
  (bind _outactors (`GameplayStatics.GetAllActorsWithTag` "LS_GameClear"))
  (for _array_element _outactors
    (bind _aslevel_sequence_actor (cast `LevelSequenceActor` _array_element))
    (bind _sequenceplayer (`LevelSequenceActor.SequencePlayer` _aslevel_sequence_actor))
    (`MovieSceneSequencePlayer.SetPlaybackPosition` _sequenceplayer (make `MovieSceneSequencePlaybackParams` (make `FrameTime` (make `FrameNumber` 0))))
    (`MovieSceneSequencePlayer.Play` _sequenceplayer)
    (add `MovieSceneSequencePlayer.OnFinished` _sequenceplayer (delegate `OnFinished(GameClear)`))
    (break)))

(event `OnFinished(GameClear)`
  (bind _asbp_game_mode (cast `/Game/Main/Common/Bluprints/BP_GameMode` (`GameplayStatics.GetGameMode`)))
  (`GameMode.RestartGame` _asbp_game_mode))

(fn `UserConstructionScript`)