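; BP_SystemSpawnInfinity is an endless enemy spawner that respawns the same configured wave whenever its enemies are wiped out.
; SpawnWave spawns each valid enemy class in WaveInfo at its target actor's transform, gives it a default controller, sets its SpawnType and increments the field count.
; DecreaseEnemyCount, meant to be called on enemy death, decrements that count and calls SpawnWave after a short delay at zero.
; BeginPlay only resets the count.
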(event `self.ReceiveBeginPlay`
  (set `self.FieldEnemyCount` 0) ; レベル上の敵の数初期化
)

(event `DecreaseEnemyCount`
  ;[1 1 1] 敵カウントを1減少させる
  (bind _result (`/Engine/EditorBlueprintResources/StandardMacros.DecrementInt` (`self.FieldEnemyCount`))
    (:`  `
      ;[1 1 1] レベル上に敵が存在しなくなったら、敵を生成する
      (if (== _result 0)
        (`KismetSystemLibrary.Delay` 3.0)
        (`self.SpawnWave`)))))

(event `SpawnWave`
  (`|ExecutionSequence`
    (:`then_0`
      ;[1 1 1] 指定された配列番号のウェーブを呼び出し、敵を生成する(レベル上の敵をループ分増加させる)
      (for _array_element (`/Game/Features/System/Blueprints/SpawnWave/BP_WaveInfo.SpawnEnemyInfo` (`self.WaveInfo`))
        (bind (_enemytype _enemytransformtarget) (break `/Game/Features/System/Blueprints/SpawnWave/ST_SpawnEnemyInfo` _array_element))
        (if (`KismetSystemLibrary.IsValidClass` _enemytype)
          (if (`KismetSystemLibrary.IsValid` _enemytransformtarget)
            (bind _returnvalue (`|SpawnActorFromClass` _enemytype (`self.GetTransform` _enemytransformtarget) "Undefined" "OverrideRootScale" null null))
            (`Pawn.SpawnDefaultController` _returnvalue)
            (`/Engine/EditorBlueprintResources/StandardMacros.IncrementInt` (`self.FieldEnemyCount`)
              (:`  `
                (set `/Game/Features/Enemy/CBP_BaseEnemy.SpawnType` "NewEnumerator2" _returnvalue)))))))))

(fn `UserConstructionScript`)