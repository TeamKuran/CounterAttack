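; AI controller for the far variant of the ZakoC enemy, driving its behavior and player detection.
; On BeginPlay it sets up the BB_ZakoC_Far blackboard and runs the BT_ZakoC_Far behavior tree.
; When perception updates include the player character, it copies whether the first last-sensed stimulus succeeded into the SensedFlag blackboard key.
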(event `self.ReceiveBeginPlay`
  (`self.UseBlackboard` "/Game/Features/NewZako/ZakoC/アセット/BB_ZakoC_Far.BB_ZakoC_Far")
  (`self.RunBehaviorTree` "/Game/Features/NewZako/ZakoC/アセット/BT_ZakoC_Far.BT_ZakoC_Far"))

(event `self.AIPerception.OnPerceptionUpdated`
  (params (UpdatedActors :type "Array of Actor Object Reference (by ref)"))
  (for _array_element UpdatedActors
    (if (== _array_element (`GameplayStatics.GetPlayerCharacter` 0))
      (bind _info (`AIPerceptionComponent.GetActorsPerception` (`self.AIPerception`) _array_element))
      (`BlackboardComponent.SetValueAsBool` (`AIBlueprintHelperLibrary.GetBlackboard` self) "SensedFlag" (`.bSuccessfullySensed` (break `AIStimulus` (`|GetArrayItem` (`.LastSensedStimuli` (break `ActorPerceptionBlueprintInfo` _info)))))))))

(fn `UserConstructionScript`)