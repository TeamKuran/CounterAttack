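; Base character Blueprint for players, managing health, timed combat states and charge timing, with stub functions for normal, special and three-tier charge attacks.
; Damage, heal and init functions set health and refresh the HP bar widget, with damage also updating the alive flag.
; Tick counts down invincibility, hit-back and super-armor timers set by Add functions, and accumulates charge time while charging.
; Invincibility combines the timed flag with a direct flag.
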(event EventBeginPlay
  (Variables|Health|SetCurHealth (Variables|Health|GetMaxHealth)))

(event Collision|EventActorBeginOverlap
  (params (OtherActor :type Actor%20Object%20Reference)))

(event EventTick
  (params (DeltaSeconds :type Float%20%28single-precision%29))
  (Utilities|FlowControl|Sequence
    (:then_0
      (State|UpdateInvicible DeltaSeconds))
    (:then_1
      (State|UpdateHitBack DeltaSeconds))
    (:then_2
      (State|UpdateSuperArmer DeltaSeconds))
    (:then_3
      (State|AddChargeingTime DeltaSeconds))))

(fn ConstructionScript)

(fn UpdateHealthBar
  ;[1 1 1] Healthバー更新
  (Default|UpdateHP (Variables|Health|GetWBP_HPBarRef) (|({03BD4930-4ABC-52D7-EB0D-DEA1B9A1D18C}/{6F50901B-4E75-4740-00FA-91964FB8535D}))))

(fn HealHealth
  (params (Value :type Float%20%28single-precision%29))
  ;[1 1 1] ヘルス回復
  (Variables|Health|SetCurHealth (|(min(({03BD4930-4ABC-52D7-EB0D-DEA1B9A1D18C}+Value),{6F50901B-4E75-4740-00FA-91964FB8535D})) Value))
  (Health|UpdateHealthBar))

(fn DamageHealth
  (params (Value :type Float%20%28single-precision%29))
  ;[1 1 1] ヘルスにダメージ
  (Variables|Health|SetCurHealth (|(max(({03BD4930-4ABC-52D7-EB0D-DEA1B9A1D18C}-Value))) Value))
  (Health|UpdateHealthBar)
  (Variables|Health|SetisAlive (> (Variables|Health|GetCurHealth) 0.0)))

(fn InitHealth
  ;[1 1 1] ヘルス初期化
  (Variables|Health|SetCurHealth (Variables|Health|GetMaxHealth))
  (Health|UpdateHealthBar))

(fn UpdateInvicible
  (params (DeltaSeconds :type Float%20%28single-precision%29))
  (Utilities|FlowControl|Sequence
    (:then_0
      ;[1 1 1] 無敵時間によるフラグ管理
      (if (Variables|State|GetInvicibbleFlg%28Time%29)
        (Variables|State|SetInvicibleTime (|(max(({C8A5E42D-48AC-FD0A-4210-E8B80511A888}-DeltaSeconds))) DeltaSeconds))
        (if (>= 0.0 (Variables|State|GetInvicibleTime))
          (Variables|State|SetInvicibbleFlg%28Time%29 false))))
    (:then_1
      ;[1 1 1] 無敵状態を更新
      (Variables|State|SetInvicibleFlg (or (Variables|State|GetInvicibbleFlg%28Time%29) (Variables|State|GetInvicibleFlg%28Direct%29))))))

(fn UpdateHitBack
  (params (DeltaSeconds :type Float%20%28single-precision%29))
  ;[1 1 1] のけぞり時間とフラグ更新
  (if (Variables|State|GetHitBackFlg)
    (Variables|State|SetHitBackTime (|(max(({AEA148F7-4CBB-4963-A3C1-7483BA762845}-DeltaSeconds))) DeltaSeconds))
    (if (>= 0.0 (Variables|State|GetHitBackTime))
      (Variables|State|SetHitBackFlg false))))

(fn UpdateSuperArmer
  (params (DeltaSeconds :type Float%20%28single-precision%29))
  ;[1 1 1] スーパーアーマー時間とフラグ更新
  (if (Variables|State|GetSuperArmerFlg)
    (Variables|State|SetSuperArmerTime (|(max(({34F3A9A5-47E2-D71F-7A98-06B1D115A0D4}-DeltaSeconds))) DeltaSeconds))
    (if (>= 0.0 (Variables|State|GetSuperArmerTime))
      (Variables|State|SetSuperArmerFlg false))))

(fn AddInvisivle
  (params (DeltaSeconds :type Float%20%28single-precision%29))
  ;[1 1 1] 無敵付与
  (Variables|State|SetInvicibleTime (|({C8A5E42D-48AC-FD0A-4210-E8B80511A888}+DeltaSeconds) DeltaSeconds))
  (Variables|State|SetInvicibbleFlg%28Time%29 true))

(fn AddHitBack
  (params (DeltaSeconds :type Float%20%28single-precision%29))
  ;[1 1 1] 無敵付与
  (Variables|State|SetHitBackTime (|({AEA148F7-4CBB-4963-A3C1-7483BA762845}+DeltaSeconds) DeltaSeconds))
  (Variables|State|SetHitBackFlg true))

(fn AddSuperArmer
  (params (DeltaSeconds :type Float%20%28single-precision%29))
  ;[1 1 1] スーパーアーマー付与
  (Variables|State|SetSuperArmerTime (|({34F3A9A5-47E2-D71F-7A98-06B1D115A0D4}+DeltaSeconds) DeltaSeconds))
  (Variables|State|SetSuperArmerFlg true))

(fn NormalAttack)

(fn ThirdChargeAttack
  (return 0.0))

(fn SpecialAttack)

(fn SecondChargeAttack
  (return 0.0))

(fn FirstChargeAttack
  (return 0.0))

(fn StartChargeing
  (Variables|State|SetChargeingFlg true))

(fn ResetChargeing
  (Variables|State|SetChargeingFlg false))

(fn AddChargeingTime
  (params (DeltaSeconds :type Float%20%28single-precision%29))
  (if (Variables|State|GetChargeingFlg)
    (Variables|State|SetChargeingTime (|({85B74AC1-487B-DA87-0D38-50931419756F}+DeltaSeconds) DeltaSeconds))
    (else
      (Variables|State|SetChargeingTime 0.0))))