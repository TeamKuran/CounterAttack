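; BP_BaseWeapon is a weapon actor that damages damageable actors, other than its owner, overlapping its sword collision.
; SwordActive and SwordDeactive toggle that collision, intended for AnimNotify calls.
; Player-owned hits feed the boss counter gauge, then damage only non-invincible BP_BaseEnemy targets, while other owners skip both checks.
; Damaging hits spawn a burst effect, play a sound and, when flagged, trigger a one-shot FlyAway on the target.
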(event `self.SwordCollision.OnComponentBeginOverlap`
  (params (OverlappedComponent :type "PrimitiveComponent Object Reference") (OtherActor :type "Actor Object Reference") (OtherComp :type "PrimitiveComponent Object Reference") (OtherBodyIndex :type Integer) (bFromSweep :type Boolean) (SweepResult :type "HitResult Structure (by ref)"))
  (bind _returnvalue (`self.GetOwner`))
  ;[1 1 1] overlapした時に自分の親アクタ以外だった場合、applydamageで敵にダメージを与える
  (if (!= OtherActor _returnvalue)
    (if (`Actor.bCanBeDamaged` OtherActor)
      (bind _astest_player_bp (cast `/Game/Features/Player/Blueprints/TestPlayer_BP` (`self.GetOwner`))
        (:`then`
          ;[1 1 1] 持ち主がプレイヤーの場合の処理
          (`/Game/Features/UI/Blueprints/System/UI/Counter/WBP_CounterGage.AddBossCounterGage` (`/Game/Features/Player/Blueprints/TestPlayer_BP.BossCoounterGage` _astest_player_bp) (`self.AddBossGageValue`))
          (bind _asbp_base_enemy (cast `/Game/Features/Enemy/BP_BaseEnemy` OtherActor))
          (if (not (`/Game/Features/Enemy/BP_BaseEnemy.InviFlag` _asbp_base_enemy))
            (`GameplayStatics.ApplyDamage` OtherActor (`self.SwordDamage`) null self :!label _label)
            (`NiagaraFunctionLibrary.SpawnSystemAtLocation` "/Game/Main/Common/Niagara/HitEffect/FX/FX_Burst.FX_Burst" (`self.K2_GetActorLocation`))
            (if (`self.FlyAway`)
              (`/Game/Features/Player/MacroLiblary/Macro.FlyAway` OtherActor _returnvalue
                (:`Out`
                  (set `self.FlyAway` false))))
            (`GameplayStatics.PlaySound2D` "/Game/Main/Common/Sound/SE/Cut01-1__online-audio-converter_com_.Cut01-1__online-audio-converter_com_" 1.0 1.0 0.0 null null)
            (`KismetSystemLibrary.Delay` 0.5)))
        (:`CastFailed`
          (goto _label))))))

(event `SwordActive`
  ;[1 1 1] SwordCollisionを有効無効を切り替える.Animnotifyで使用するカスタムイベント
  (`PrimitiveComponent.SetCollisionProfileName` (`self.SwordCollision`) "OverlapAll" true))

(event `SwordDeactive`
  ;[1 1 1] SwordCollisionを有効無効を切り替える.Animnotifyで使用するカスタムイベント
  (`PrimitiveComponent.SetCollisionEnabled` (`self.SwordCollision`) "NoCollision"))

(fn `UserConstructionScript`)