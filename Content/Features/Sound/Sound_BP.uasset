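; Actor Blueprint that drives a keyboard-controlled sound options menu.
; It creates WBP_SoundOption on BeginPlay; P adds it to the viewport with the mouse cursor, and K removes it.
; Up and Down wrap a selection index across four entries and mirror it to the widget.
; Left and Right pass that index to the widget's volume functions; Enter on the last entry closes the menu and resets selection.
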(event `self.ReceiveBeginPlay`
  ;[1 1 1] Widgetの作成・変数に格納
  (bind _returnvalue (`|CreateWidget` "/Game/Features/Sound/WBP_SoundOption.WBP_SoundOption_C"))
  (bind _output_get (set `self.WBPSoundOption` _returnvalue))
  (set `/Game/Features/Sound/WBP_SoundOption.SoundOption` _output_get (`self.WBPSoundOption`)))

(event `Key|Right` :consume false
  (params (Key :type "Key Structure"))
  ;[1 1 1] キーボード
  (:`Pressed`
    (`/Game/Features/Sound/WBP_SoundOption.RKeyBoardMasterVolume` (`self.WBPSoundOption`) (`self.SelectNum`))))

(event `Key|Up` :consume false
  (params (Key :type "Key Structure"))
  (bind _returnvalue (- (`self.SelectNum`) 1))
  ;[1 1 1] キーボード
  (:`Pressed`
    (if (<= _returnvalue -1)
      (bind _output_get (set `self.SelectNum` 3))
      (set `/Game/Features/Sound/WBP_SoundOption.PosNum` _output_get (`self.WBPSoundOption`))
      (else
        (bind _output_get_2 (set `self.SelectNum` _returnvalue))
        (set `/Game/Features/Sound/WBP_SoundOption.PosNum` _output_get_2 (`self.WBPSoundOption`))))))

(event `Key|P` :consume false
  (params (Key :type "Key Structure"))
  ;[1 1 1] Widgetの取付
  (:`Pressed`
    (`UserWidget.AddToViewport` (`self.WBPSoundOption`) 0)
    (set `PlayerController.bShowMouseCursor` true (`GameplayStatics.GetPlayerController` 0))))

(event `Key|Left` :consume false
  (params (Key :type "Key Structure"))
  ;[1 1 1] キーボード
  (:`Pressed`
    (`/Game/Features/Sound/WBP_SoundOption.LKeyBoardMasterVolume` (`self.WBPSoundOption`) (`self.SelectNum`))))

(event `Key|Down` :consume false
  (params (Key :type "Key Structure"))
  (bind _returnvalue (+ (`self.SelectNum`) 1))
  ;[1 1 1] キーボード
  (:`Pressed`
    (if (>= _returnvalue 4)
      (bind _output_get (set `self.SelectNum` 0))
      (set `/Game/Features/Sound/WBP_SoundOption.PosNum` _output_get (`self.WBPSoundOption`))
      (else
        (bind _output_get_2 (set `self.SelectNum` _returnvalue))
        (set `/Game/Features/Sound/WBP_SoundOption.PosNum` _output_get_2 (`self.WBPSoundOption`))))))

(event `Key|Enter` :consume false
  (params (Key :type "Key Structure"))
  ;[1 1 1] キーボード
  (:`Pressed`
    (if (== (`self.SelectNum`) 3)
      (`/Game/Features/Sound/WBP_SoundOption.WidgetErase` (`self.WBPSoundOption`))
      (set `self.SelectNum` 0)
      (set `/Game/Features/Sound/WBP_SoundOption.PosNum` 0 (`self.WBPSoundOption`)))))

(event `Key|K` :consume false
  (params (Key :type "Key Structure"))
  ;[1 1 1] Widgetの取り除く
  (:`Pressed`
    (`/Game/Features/Sound/WBP_SoundOption.WidgetErase` (`self.WBPSoundOption`))))

(fn `UserConstructionScript`)