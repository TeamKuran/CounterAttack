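; Select_BP is a title-scene actor that forwards key presses to a start UI widget.
; Tick re-enables input from player controller 0 every frame, and pressing U or M calls SNum on the StartUI reference.
; The logic that creates WEB_StartUI_BP, stores it in StartUI, shows the cursor and adds it to the screen is disconnected, so this graph never assigns that reference.
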(event `self.ReceiveBeginPlay`)

(event `Key|U`
  (params (Key :type "Key Structure"))
  (:`Pressed`
    (`/Game/Features/Scene/Title/アセット/WEB_StartUI_BP.SNum+` (`self.StartUI`))))

(event `self.ReceiveTick`
  (params (DeltaSeconds :type "Float (single-precision)"))
  (`self.EnableInput` (`GameplayStatics.GetPlayerController` 0)))

(event `Key|M`
  (params (Key :type "Key Structure"))
  (:`Pressed`
    (`/Game/Features/Scene/Title/アセット/WEB_StartUI_BP.SNum-` (`self.StartUI`))))

(fn `UserConstructionScript`)