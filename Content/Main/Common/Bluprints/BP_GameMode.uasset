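; BP_GameMode is a game mode Blueprint that sets up the HUD widgets for player HP, boss HP and a counter gauge.
; On BeginPlay it creates each widget, stores it in a variable and adds it to the viewport.
; All three start invisible, with the boss bar Collapsed and the other two Hidden, and nothing here reveals them.
; AddCounterGage is an empty stub.
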(event `self.ReceiveBeginPlay`
  (`|ExecutionSequence`
    (:`then_0`
      (bind _returnvalue (`|CreateWidget` "/Game/Features/UI/Blueprints/Player/UMG_HPBar_Player.UMG_HPBar_Player_C"))
      (bind _output_get (set `self.HPBarPlayerWidget` _returnvalue))
      (`UserWidget.AddToViewport` _output_get 0)
      (`Widget.SetVisibility` _output_get "Hidden"))
    (:`then_1`
      (bind _returnvalue_2 (`|CreateWidget` "/Game/Features/UI/Blueprints/Enemy/WBP_HPBar_Boss.WBP_HPBar_Boss_C"))
      (bind _output_get_2 (set `self.HPBarBossWidget` _returnvalue_2))
      (`UserWidget.AddToViewport` _output_get_2 0)
      (`Widget.SetVisibility` _output_get_2 "Collapsed"))
    (:`then_2`
      (bind _returnvalue_3 (`|CreateWidget` "/Game/Features/UI/Blueprints/Counter/UMG_CounterGauge.UMG_CounterGauge_C"))
      (bind _output_get_3 (set `self.CounterGageWidget` _returnvalue_3))
      (`UserWidget.AddToViewport` _output_get_3 0)
      (`Widget.SetVisibility` _output_get_3 "Hidden"))))

(fn `AddCounterGage`
  (params (NewParam :type Integer)))

(fn `UserConstructionScript`)